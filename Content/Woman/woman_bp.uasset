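; Woman character Blueprint for an AI-controlled NPC that moves away from a spotted location.
; Spotted raises walk speed and uses SimpleMoveToLocation to head directly opposite the given location, unless StartTurn is set.
; BeginPlay binds to the MoveAround AI controller's move-completed event, which restores the slower walk speed and clears StartTurn once velocity is zero.
; Incremental turning and angled-flee logic remains in the graph but is disconnected.
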(event Custom|Spotted
  (params (Location :type Vector))
  (bind _returnvalue (Transformation|GetActorLocation))
  (if (not (Variables|Default|GetstartTurn))
    (Variables|/Script/Engine.CharacterMovementComponent|SetMaxWalkSpeed (Variables|Character|GetCharacterMovement) 1.2e+02)
    (AI|Navigation|SimpleMovetoLocation (AI|GetAIController self) (+ _returnvalue (- _returnvalue Location)))))

(event Custom|reset%20speed
  (params (RequestID :type AI%20Request%20ID%20Structure) (Result :type EPathFollowingResult%20Enum :default "Success"))
  (if (== (Math|Vector|VectorLength (Transformation|GetVelocity)) 0.0)
    (Variables|/Script/Engine.CharacterMovementComponent|SetMaxWalkSpeed (Variables|Character|GetCharacterMovement) 9e+01)
    (Variables|Default|SetstartTurn false)))

(event EventBeginPlay
  (bind _asmove_around (Utilities|Casting|CastToMoveAround (AI|GetAIController self)))
  (EventDispatchers|BindEventtoReceiveMoveCompleted _asmove_around (delegate Custom|reset%20speed)))

(event Collision|EventActorBeginOverlap
  (params (OtherActor :type Actor%20Object%20Reference)))

(event EventTick
  (params (DeltaSeconds :type Float%20%28single-precision%29)))

(fn ConstructionScript)